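; Base power-up pickup actor that changes the walk speed of a Character that touches it.
; The configurable PowerUpMesh is applied to ItemMesh in both the Construction Script and BeginPlay.
; On overlap, it sets the Character's MaxWalkSpeed to NewMaxWalkSpeed, prints PickupMessage and destroys itself.
; The speed change has no timer or reset here, and Tick is unused.
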(event EventBeginPlay
  (Components|StaticMesh|SetStaticMesh (Variables|Default|GetItemMesh) (Variables|Default|GetPowerUpMesh)))

(event Collision|EventActorBeginOverlap
  (params (OtherActor :type Actor%20Object%20Reference))
  (bind _ascharacter (Utilities|Casting|CastToCharacter OtherActor))
  (Variables|/Script/Engine.CharacterMovementComponent|SetMaxWalkSpeed (Variables|/Script/Engine.Character|GetCharacterMovement _ascharacter) (Variables|Default|GetNewMaxWalkSpeed))
  (Development|PrintString (Variables|Default|GetPickupMessage))
  (Actor|DestroyActor))

(event EventTick
  (params (DeltaSeconds :type Float%20%28single-precision%29)))

(fn ConstructionScript
  (Components|StaticMesh|SetStaticMesh (Variables|Default|GetItemMesh) (Variables|Default|GetPowerUpMesh)))